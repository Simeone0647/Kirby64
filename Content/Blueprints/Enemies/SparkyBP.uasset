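; SparkyBP is an enemy that damages the player on contact.
; When its Hitbox overlaps a component tagged Hurtbox on an actor tagged Player, it deals one damage through that actor's Life component and plays two 2D hit sounds.
; Its Sparks component is deactivated at BeginPlay, and nothing in this graph turns it back on.
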(event OnComponentBeginOverlap(Hitbox)
  (params (OverlappedComponent :type Primitive%20Component%20Object%20Reference) (OtherActor :type Actor%20Object%20Reference) (OtherComp :type Primitive%20Component%20Object%20Reference) (OtherBodyIndex :type Integer) (bFromSweep :type Boolean) (SweepResult :type Hit%20Result%20Structure%20%28by%20ref%29))
  (bind _returnvalue (Actor|GetComponentbyClass OtherActor "/Script/Kirby64.Life"))
  (if (Math|Boolean|ANDBoolean (Utilities|IsValid OtherComp) (Actor|ActorHasTag OtherActor "Player") (Components|ComponentHasTag OtherComp "Hurtbox"))
    (if (Utilities|IsValid _returnvalue)
      (Class|Life|DoDamage _returnvalue 1)
      (Audio|PlaySound2D "/Game/Sounds/Effects/Kirby/KirbyHitted.KirbyHitted" 1.0 1.0 0.0 0 0)
      (Audio|PlaySound2D "/Game/Sounds/Effects/Kirby/Hit.Hit" 1.5 1.0 0.0 0 0))))

(event EventBeginPlay
  (Components|Activation|Deactivate (Variables|Default|GetSparks)))

(fn ConstructionScript)