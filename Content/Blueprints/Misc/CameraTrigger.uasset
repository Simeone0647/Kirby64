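; Trigger volume that gradually changes the side-scroller player's camera boom rotation and socket offset as they move through it.
; On overlap it stores the current boom settings, takes the farther Y end of the box as the target, and records the distance to it.
; Tick blends toward that side's left or right camera settings as the player nears the target.
; Leaving clears the tracking state without restoring the camera.
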(event OnComponentBeginOverlap(Box)
  (params (OverlappedComponent :type Primitive%20Component%20Object%20Reference) (OtherActor :type Actor%20Object%20Reference) (OtherComp :type Primitive%20Component%20Object%20Reference) (OtherBodyIndex :type Integer) (bFromSweep :type Boolean) (SweepResult :type Hit%20Result%20Structure%20%28by%20ref%29))
  (bind _returnvalue (Transformation|GetActorLocation))
  (bind _box (Variables|Default|GetBox))
  (bind _returnvalue_2 (Components|Box|GetScaledBoxExtent _box))
  (bind _y (Math|Vector|BreakVector _returnvalue_2))
  (bind _returnvalue_3 (Math|Vector|MakeVector 0.0 _y 0.0))
  (bind _returnvalue_4 (- _returnvalue _returnvalue_3))
  (bind _returnvalue_5 (+ _returnvalue _returnvalue_3))
  (if (Actor|ActorHasTag OtherActor "Player")
    (bind _asside_scroller_character (Utilities|Casting|CastToSideScrollerCharacter OtherActor))
    (Variables|Default|SetMainCharRef _asside_scroller_character)
    (if (< (Math|Vector|Distance(Vector) (Transformation|GetActorLocation _asside_scroller_character) _returnvalue_5) (Math|Vector|Distance(Vector) (Transformation|GetActorLocation _asside_scroller_character) _returnvalue_4))
      (Variables|Default|SetMaxDistance (Math|Vector|Distance(Vector) (Transformation|GetActorLocation _asside_scroller_character) _returnvalue_4))
      (Variables|Default|SetLeftPoint _returnvalue_4)
      (else
        (Variables|Default|SetMaxDistance (Math|Vector|Distance(Vector) (Transformation|GetActorLocation _asside_scroller_character) _returnvalue_5))
        (Variables|Default|SetRightPoint _returnvalue_5)))
    (Variables|Default|SetOriginalCameraRotation (Transformation|GetWorldRotation (Variables|/Script/Kirby64.Kirby64Character|GetCameraBoom (Variables|Default|GetMainCharRef))))
    (Variables|Default|SetOriginalBoomSocketOffset (Variables|/Script/Engine.SpringArmComponent|GetSocketOffset (Variables|/Script/Kirby64.Kirby64Character|GetCameraBoom (Variables|Default|GetMainCharRef))))))

(event OnComponentEndOverlap(Box)
  (params (OverlappedComponent :type Primitive%20Component%20Object%20Reference) (OtherActor :type Actor%20Object%20Reference) (OtherComp :type Primitive%20Component%20Object%20Reference) (OtherBodyIndex :type Integer))
  (if (Actor|ActorHasTag OtherActor "Player")
    (Variables|Default|SetMaxDistance 0.0)
    (Variables|Default|SetMainCharRef 0)
    (Variables|Default|SetLeftPoint "0, 0, 0")
    (Variables|Default|SetRightPoint "0, 0, 0")))

(event EventTick
  (params (DeltaSeconds :type Float%20%28single-precision%29))
  (bind _maincharref (Variables|Default|GetMainCharRef))
  (bind _maxdistance (Variables|Default|GetMaxDistance))
  (bind _maincharref_2 (Variables|Default|GetMainCharRef))
  (bind _maxdistance_2 (Variables|Default|GetMaxDistance))
  (bind _leftpoint (Variables|Default|GetLeftPoint))
  (bind _rightpoint (Variables|Default|GetRightPoint))
  (bind _maincharref_3 (Variables|Default|GetMainCharRef))
  (bind _returnvalue (Transformation|GetActorLocation _maincharref))
  (bind _returnvalue_2 (Transformation|GetActorLocation _maincharref_2))
  (bind _returnvalue_3 (Math|Vector|Distance(Vector) _returnvalue _rightpoint))
  (bind _returnvalue_4 (Math|Vector|Distance(Vector) _returnvalue_2 _leftpoint))
  (bind _returnvalue_5 (/ _returnvalue_3 _maxdistance))
  (bind _returnvalue_6 (/ _returnvalue_4 _maxdistance_2))
  (bind _returnvalue_7 (- _returnvalue_5 1.0))
  (bind _returnvalue_8 (- _returnvalue_6 1.0))
  (bind _returnvalue_9 (Math|Float|Absolute(Float) _returnvalue_7))
  (bind _returnvalue_10 (Math|Float|Absolute(Float) _returnvalue_8))
  (Utilities|IsValid _maincharref_3
    (:Is%20Valid
      (if (Class|KismetMathLibrary|NotEqualExactlyVectorVector (Variables|Default|GetLeftPoint) "0, 0, 0")
        (Default|SetBoomRotationandSocketOffset _maincharref_3 (Math|Rotator|Lerp(Rotator) (Variables|Default|GetOriginalCameraRotation) (Variables|Default|GetCameraRotationLeft) _returnvalue_10 true) (Math|Vector|Lerp(Vector) (Variables|Default|GetOriginalBoomSocketOffset) (Variables|Default|GetCameraBoomSockerOffsetLeft) _returnvalue_10))
        (else
          (Default|SetBoomRotationandSocketOffset _maincharref_3 (Math|Rotator|Lerp(Rotator) (Variables|Default|GetOriginalCameraRotation) (Variables|Default|GetCameraRotationRight) _returnvalue_9 true) (Math|Vector|Lerp(Vector) (Variables|Default|GetOriginalBoomSocketOffset) (Variables|Default|GetCameraBoomSocketOffsetRight) _returnvalue_9)))))))

(fn ConstructionScript)