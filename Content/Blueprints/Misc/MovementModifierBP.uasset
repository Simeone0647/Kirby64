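; MovementModifierBP is a trigger-box Blueprint that, despite its name, only reports the side-scroller player's velocity and modifies no movement.
; When an actor tagged Player overlaps the Box, it casts it to SideScrollerCharacter and caches it in PlayerRef.
; Tick then prints that character's velocity every frame, and nothing clears the reference, so printing continues after the player leaves the box.
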(event OnComponentBeginOverlap(Box)
  (params (OverlappedComponent :type Primitive%20Component%20Object%20Reference) (OtherActor :type Actor%20Object%20Reference) (OtherComp :type Primitive%20Component%20Object%20Reference) (OtherBodyIndex :type Integer) (bFromSweep :type Boolean) (SweepResult :type Hit%20Result%20Structure%20%28by%20ref%29))
  (if (Actor|ActorHasTag OtherActor "Player")
    (bind _asside_scroller_character (Utilities|Casting|CastToSideScrollerCharacter OtherActor))
    (Variables|Default|SetPlayerRef _asside_scroller_character)))

(event EventBeginPlay)

(event Collision|EventActorBeginOverlap
  (params (OtherActor :type Actor%20Object%20Reference)))

(event EventTick
  (params (DeltaSeconds :type Float%20%28single-precision%29))
  (if (Utilities|IsValid (Variables|Default|GetPlayerRef))
    (Development|PrintString (Utilities|String|ToString(Vector) (Transformation|GetVelocity (Variables|Default|GetPlayerRef))))))

(fn ConstructionScript)