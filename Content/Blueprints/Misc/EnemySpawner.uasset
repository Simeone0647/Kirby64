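; Enemy spawner actor that keeps one enemy alive at its location, respawning it after a delay when it is gone.
; BeginPlay spawns the configured Enemy class at the spawner's transform, gives it a default controller and sets its initial state.
; Tick accumulates time while the stored enemy reference is invalid, then repeats the same spawn and setup once SpawnTime is reached.
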(event EventBeginPlay
  (bind _returnvalue (Game|SpawnActorfromClass (Variables|Default|GetEnemy) (Transformation|GetActorTransform self) "Undefined" 0 0))
  (bind _output_get (Variables|Default|SetEnemyRef _returnvalue))
  (if (Utilities|IsValid _output_get)
    (Pawn|SpawnDefaultController _output_get)
    (Class|Enemy|SetState _output_get (Variables|Default|GetInitialState))))

(event Collision|EventActorBeginOverlap
  (params (OtherActor :type Actor%20Object%20Reference)))

(event EventTick
  (params (DeltaSeconds :type Float%20%28single-precision%29))
  (if (not (Utilities|IsValid (Variables|Default|GetEnemyRef)))
    (bind _output_get (Variables|Default|SetTimer (+ DeltaSeconds (Variables|Default|GetTimer))))
    (if (>= _output_get (Variables|Default|GetSpawnTime))
      (Variables|Default|SetTimer 0.0)
      (bind _returnvalue (Game|SpawnActorfromClass (Variables|Default|GetEnemy) (Transformation|GetActorTransform self) "Undefined" 0 0))
      (bind _output_get_2 (Variables|Default|SetEnemyRef _returnvalue))
      (if (Utilities|IsValid _output_get_2)
        (Pawn|SpawnDefaultController _output_get_2)
        (Class|Enemy|SetState _output_get_2 (Variables|Default|GetInitialState))))))

(fn ConstructionScript)